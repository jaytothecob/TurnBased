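; Non-nativized gameplay functions for the turn-based tile toolkit, holding the check that ends the game when one faction remains.
; It scans all Unit actors, skipping those pending death, to collect unique surviving factions.
; If exactly one remains, it shows the game-over screen on HUD_Faction_Turn and sets GameOver on ATBTT_GameMode.
; The win text names the current pawn's faction rather than reading the surviving faction list.
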(fn `End Game If Only One Faction Remains`
  (locals (`Remaining Factions` :type "Array of /Game/AdvancedTurnBasedTileToolkit/Blueprints/Gameplay/Enums/Enum_Faction Enum"))
  (`KismetArrayLibrary.Array_Clear` (`local.Remaining Factions`))
  (bind _outactors (`GameplayStatics.GetAllActorsOfClass` null "/Game/AdvancedTurnBasedTileToolkit/Blueprints/Pawns/Unit.Unit_C"))
  (for _array_element _outactors
    (if (not (`/Game/AdvancedTurnBasedTileToolkit/Blueprints/Pawns/Unit.Pending Death` _array_element))
      (`KismetArrayLibrary.Array_AddUnique` (`local.Remaining Factions`) (`/Game/AdvancedTurnBasedTileToolkit/Blueprints/Pawns/Unit.Faction` _array_element))))
  (if (== (`KismetArrayLibrary.Array_Length` (`local.Remaining Factions`)) 1)
    (bind _foundwidgets (`WidgetBlueprintLibrary.GetAllWidgetsOfClass` null "/Game/AdvancedTurnBasedTileToolkit/Blueprints/Gameplay/HUD_Faction_Turn.HUD_Faction_Turn_C"))
    (bind _output (`|GetArrayItem` _foundwidgets))
    (`TextBlock.SetText` (`/Game/AdvancedTurnBasedTileToolkit/Blueprints/Gameplay/HUD_Faction_Turn.text_game_over` _output) (`KismetTextLibrary.Conv_StringToText` (`KismetStringLibrary.Concat_StrStr` (`KismetStringLibrary.ToUpper` (`|GetEnumeratorNameAsString` (`/Game/AdvancedTurnBasedTileToolkit/Blueprints/Pawns/Unit.Faction` (`/Game/AdvancedTurnBasedTileToolkit/Blueprints/Gameplay/ATBTT_GameMode.CurrentPawn` (cast `/Game/AdvancedTurnBasedTileToolkit/Blueprints/Gameplay/ATBTT_GameMode` (`GameplayStatics.GetGameMode` null) :!pure true))))) " FACTION WINS!")))
    (`/Game/AdvancedTurnBasedTileToolkit/Blueprints/Gameplay/HUD_Faction_Turn.Game Over HUD` _output)
    (set `/Game/AdvancedTurnBasedTileToolkit/Blueprints/Gameplay/ATBTT_GameMode.Game Over` true (cast `/Game/AdvancedTurnBasedTileToolkit/Blueprints/Gameplay/ATBTT_GameMode` (`GameplayStatics.GetGameMode` null) :!pure true))
    (return)
    (else
      (return))))