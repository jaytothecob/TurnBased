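; Player melee scout pawn for the turn-based tile toolkit that adds skeletal animation to inherited unit behaviour.
; Move, attack and kill events run parent logic, then call matching animations on the mesh's Pawn_Anim_BP_Parent instance.
; Move updates call MoveAnimation continuously while not Idle, clearing Break and resetting a DoOnce that limits the call while Idle.
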(event `self.ReceiveBeginPlay`
  (`parent.ReceiveBeginPlay`))

(event `self.Move Timeline__UpdateFunc`
  (bind _aspawn_anim_bp_parent (cast `/Game/AdvancedTurnBasedTileToolkit/Animations/Pawn_Anim_BP_Parent` (`SkeletalMeshComponent.GetAnimInstance` (`self.SkeletalMesh`)) :!pure true))
  (`parent.Move Timeline__UpdateFunc`)
  (if (`self.Idle`)
    (`/Engine/EditorBlueprintResources/StandardMacros.DoOnce` true :!label _label
      (:`Completed`
        _))
    (else
      (`|ExecutionSequence`
        (:`then_0`
          (goto _label :!via `Reset`))
        (:`then_1`
          (set `/Game/AdvancedTurnBasedTileToolkit/Animations/Pawn_Anim_BP_Parent.Break` false _aspawn_anim_bp_parent)))))
  (`/Game/AdvancedTurnBasedTileToolkit/Animations/Pawn_Anim_BP_Parent.MoveAnimation` _aspawn_anim_bp_parent))

(event `self.Attack Victim`
  (params (Victim :type "/Game/AdvancedTurnBasedTileToolkit/Blueprints/Pawns/Unit Object Reference"))
  (`parent.Attack Victim` Victim)
  (bind _aspawn_anim_bp_parent (cast `/Game/AdvancedTurnBasedTileToolkit/Animations/Pawn_Anim_BP_Parent` (`SkeletalMeshComponent.GetAnimInstance` (`self.SkeletalMesh`))))
  (`/Game/AdvancedTurnBasedTileToolkit/Animations/Pawn_Anim_BP_Parent.AttackAnimation` _aspawn_anim_bp_parent))

(event `self.Kill Unit`
  (params (`Anim Delay` :type "Float (single-precision)"))
  (`parent.Kill Unit` `Anim Delay`)
  (bind _aspawn_anim_bp_parent (cast `/Game/AdvancedTurnBasedTileToolkit/Animations/Pawn_Anim_BP_Parent` (`SkeletalMeshComponent.GetAnimInstance` (`self.SkeletalMesh`))))
  (`/Game/AdvancedTurnBasedTileToolkit/Animations/Pawn_Anim_BP_Parent.DeathAnimation` _aspawn_anim_bp_parent))

(fn `UserConstructionScript`
  (`parent.UserConstructionScript`))